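; Exhibition character Blueprint that adds visual and controller feedback for the movement states of its ExhibitionMovementComponent.
; Tick spawns a smoke emitter at the actor's location on every frame the component is sliding.
; Hook and rope enter/exit events start and stop force feedback on the local viewing player controller.
; Slide enter/exit and dive events are empty, and an eject sound call is left unconnected.
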(event OnEnterSlide(ExhibitionMovementComponent))

(event OnExitSlide(ExhibitionMovementComponent))

(event OnDive(ExhibitionMovementComponent))

(event OnEnterHook(ExhibitionMovementComponent)
  (bind _returnvalue (Pawn|GetLocalViewingPlayerController))
  (Utilities|IsValid _returnvalue
    (:Is%20Valid
      (Game|Feedback|ClientPlayForceFeedback _returnvalue "/Game/Game/Assets/Feedbacks/FF_HookFeedback.FF_HookFeedback" "None" false false false))))

(event OnExitHook(ExhibitionMovementComponent)
  (bind _returnvalue (Pawn|GetLocalViewingPlayerController))
  (Utilities|IsValid _returnvalue
    (:Is%20Valid
      (Game|Feedback|ClientStopForceFeedback _returnvalue "/Game/Game/Assets/Feedbacks/FF_HookFeedback.FF_HookFeedback" "None"))))

(event OnEnterRope(ExhibitionMovementComponent)
  (bind _returnvalue (Pawn|GetLocalViewingPlayerController))
  (Utilities|IsValid _returnvalue
    (:Is%20Valid
      (Game|Feedback|ClientPlayForceFeedback _returnvalue "/Game/Game/Assets/Feedbacks/FF_RopeFeedback.FF_RopeFeedback" "None" false false false))))

(event OnExitRope(ExhibitionMovementComponent)
  (bind _returnvalue (Pawn|GetLocalViewingPlayerController))
  (Utilities|IsValid _returnvalue
    (:Is%20Valid
      (Game|Feedback|ClientStopForceFeedback _returnvalue "/Game/Game/Assets/Feedbacks/FF_RopeFeedback.FF_RopeFeedback" "None"))))

(event EventBeginPlay)

(event Collision|EventActorBeginOverlap
  (params (OtherActor :type Actor%20Object%20Reference)))

(event EventTick
  (params (DeltaSeconds :type Float%20%28single-precision%29))
  (if (Class|ExhibitionMovementComponent|IsSliding (Variables|Default|GetExhibitionMovementComponent))
    (Effects|SpawnEmitteratLocation "/Game/Game/Assets/VFX/P_Smoke_Trimmed.P_Smoke_Trimmed" (Transformation|GetActorLocation))))

(fn ConstructionScript)